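; BP_Enemy_Turret is a 2D platformer enemy turret that fires bullets on a repeating timer.
; On Tick, a CanFire flag gates spawning BP_Bullet_enemy at the Scene component's world transform, then a Delay of DelayFire re-arms it.
; The turret destroys itself when a BP_Bullet overlaps it.
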(event EventBeginPlay)

(event Collision|EventActorBeginOverlap
  (params (OtherActor :type Actor%20Object%20Reference))
  (Utilities|Casting|CastToBP_Bullet OtherActor)
  (Actor|DestroyActor))

(event EventTick
  (params (DeltaSeconds :type Float%20%28single-precision%29))
  (if (Variables|Default|Getcan%20fire)
    (Variables|Default|Setcan%20fire false)
    (Game|SpawnActorfromClass "/Game/00_Platform_2D/BP_Bullet_enemy.BP_Bullet_enemy_C" (Transformation|GetWorldTransform (Variables|Default|GetScene)) "Undefined" "MultiplyWithRoot" 0 0)
    (Utilities|FlowControl|Delay (Variables|Default|GetdelayFire))
    (Variables|Default|Setcan%20fire true)))

(fn ConstructionScript)